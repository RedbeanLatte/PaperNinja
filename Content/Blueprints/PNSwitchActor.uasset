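; Floor switch actor that sinks when a Player-tagged actor enters its box trigger and signals its on and off states.
; A timeline lowers the mesh, then on finishing fires OnTurnedOn or OnTurnedOff by direction and tints a dynamic material green or red.
; The timeline reverses through TurnOff, or when any overlap ends if IsMomentary is set, as end overlap has no tag check.
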(event `self.ReceiveBeginPlay`
  (bind _returnvalue (`PrimitiveComponent.CreateDynamicMaterialInstance` (`self.Mesh`) 0 "/Game/Props/Materials/MI_Switch.MI_Switch" "None"))
  (bind _output_get (set `self.MeshMID` _returnvalue))
  (`MaterialInstanceDynamic.SetVectorParameterValue` _output_get "Tint Base Color" (struct :`R` 1.0 :`A` 1.0)))

(event `self.BoxTrigger.OnComponentBeginOverlap`
  (params (OverlappedComponent :type "PrimitiveComponent Object Reference") (OtherActor :type "Actor Object Reference") (OtherComp :type "PrimitiveComponent Object Reference") (OtherBodyIndex :type Integer) (bFromSweep :type Boolean) (SweepResult :type "HitResult Structure (by ref)"))
  (bind _meshmid (`self.MeshMID`))
  (if (`self.ActorHasTag` OtherActor "Player")
    (bind (_direction _alpha) (`Timeline|SwitchTimeline` :!label _label)
      (:`Update`
        (`SceneComponent.K2_SetRelativeLocation` (`self.Mesh`) (`KismetMathLibrary.VLerp` (0.0 0.0 0.0) (0.0 0.0 -8.0) _alpha) false false))
      (:`Finished`
        (switch `ETimelineDirection` _direction
          (:`Forward`
            (`self.OnTurnedOn`)
            (`MaterialInstanceDynamic.SetVectorParameterValue` _meshmid "Tint Base Color" (struct :`G` 1.0 :`A` 1.0)))
          (:`Backward`
            (`self.OnTurnedOff`)
            (`MaterialInstanceDynamic.SetVectorParameterValue` _meshmid "Tint Base Color" (struct :`R` 1.0 :`A` 1.0))))))))

(event `self.BoxTrigger.OnComponentEndOverlap`
  (params (OverlappedComponent :type "PrimitiveComponent Object Reference") (OtherActor :type "Actor Object Reference") (OtherComp :type "PrimitiveComponent Object Reference") (OtherBodyIndex :type Integer))
  (if (`self.IsMomentary`)
    (goto _label :!via `Reverse`)))

(event `TurnOff`
  (goto _label :!via `Reverse`))

(fn `UserConstructionScript`)