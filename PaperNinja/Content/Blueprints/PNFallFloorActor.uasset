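; A falling floor actor that drops after something overlaps it, then respawns at its original spot.
; Overlapping the BoxTrigger waits briefly, enables physics on the static mesh, then destroys the actor after a further delay.
; BeginPlay caches the starting transform and binds OnDestroyed to RespawnFallFloor, which spawns a replacement there and binds that copy's OnDestroyed too.
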(event `self.ReceiveBeginPlay`
  (add `self.OnDestroyed` (delegate `RespawnFallFloor`))
  (bind _output_get (set `self.RespawnTransform` (`self.GetTransform`))))

(event `RespawnFallFloor` :!signature `self.OnDestroyed`
  (params (DestroyedActor :type "Actor Object Reference"))
  (bind _returnvalue (`|SpawnActorFromClass` "PNFallFloorActor_C" (stale `self.ReceiveBeginPlay` _output_get) "Undefined" "OverrideRootScale" null null))
  (add `self.OnDestroyed` _returnvalue (delegate `RespawnFallFloor`)))

(event `self.BoxTrigger.OnComponentBeginOverlap`
  (params (OverlappedComponent :type "PrimitiveComponent Object Reference") (OtherActor :type "Actor Object Reference") (OtherComp :type "PrimitiveComponent Object Reference") (OtherBodyIndex :type Integer) (bFromSweep :type Boolean) (SweepResult :type "HitResult Structure (by ref)"))
  (`KismetSystemLibrary.Delay` 1.0)
  (`PrimitiveComponent.SetSimulatePhysics` (`self.StaticMeshComponent`) true)
  (`KismetSystemLibrary.Delay` 5.0)
  (`self.K2_DestroyActor`))

(fn `UserConstructionScript`)